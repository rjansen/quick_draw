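; Game mode for a quick-draw duel between player and enemy, running Intro, Wait, Draw and Finished phases.
; Tick leaves Intro after a start time, waits a random delay, then enters Draw, fires DrawPhaseStarted and shows the exclamation cue.
; A successful attack defeats the opponent, hides the cue and starts a restart timer.
; Reset returns both duelists, the phase and elapsed time to their starting state.
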(event EventBeginPlay
  (bind _returnvalue (Actor|GetActorOfClass "/Game/Blueprints/BP_Exclamation.BP_Exclamation_C"))
  (Variables|Default|SetExclamation _returnvalue)
  (bind _returnvalue_2 (Actor|GetActorOfClass "/Game/Blueprints/BP_Player.BP_Player_C"))
  (Variables|Default|SetPlayer _returnvalue_2)
  (bind _returnvalue_3 (Actor|GetActorOfClass "/Game/Blueprints/BP_Enemy.BP_Enemy_C"))
  (Variables|Default|SetEnemy _returnvalue_3))

(event EventTick
  (params (DeltaSeconds :type Float%20%28single-precision%29))
  (Variables|Default|SetElapsedTime (+ DeltaSeconds (Variables|Default|GetElapsedTime)))
  (switch Utilities|FlowControl|Switch|SwitchonE_Phases (Variables|Default|GetPhase)
    (:NewEnumerator0
      (if (>= (Variables|Default|GetElapsedTime) (Variables|Default|GetStartTime))
        (Variables|Default|SetPhase "NewEnumerator1")
        (Utilities|FlowControl|Delay (Math|Random|RandomFloatinRange (Variables|Default|GetMinDrawDelay) (Variables|Default|GetMaxDrawDelay)))
        (bind _output_get (Variables|Default|SetPhase "NewEnumerator2"))
        (Default|CallDrawPhaseStarted)
        (Development|PrintString (Utilities|String|ToString(Text) (Utilities|Text|FormatText "Game Phase: {phase}" (Utilities|String|EnumtoString _output_get))))
        (Utilities|IsValid (Variables|Default|GetExclamation)
          (:Is%20Valid
            (Default|SetVisibility (Variables|Default|GetExclamation) true))
          (:Is%20Not%20Valid
            (Development|PrintString "Invalid Exclamation Reference!")))))))

(fn ConstructionScript)

(fn SetGameFinished
  (Variables|Default|SetPhase "NewEnumerator3"))

(fn AttackedSuccessfully
  (params (IsPlayer :type Boolean))
  (if IsPlayer
    (Default|Defeated (Variables|Default|GetEnemy))
    (else
      (Default|Defeated (Variables|Default|GetPlayer))))
  (Utilities|IsValid (Variables|Default|GetExclamation)
    (:Is%20Valid
      (Default|SetVisibility (Variables|Default|GetExclamation) false)
      (Utilities|Time|SetTimerbyEvent (EventDispatchers|CreateEvent :!event Reset) (Variables|Default|GetRestartDelay)))
    (:Is%20Not%20Valid
      (Development|PrintString "Invalid Exclamation Reference!"))))

(fn Reset
  (Variables|Default|SetPhase "NewEnumerator0")
  (Variables|Default|SetElapsedTime 0.0)
  (Default|Reset (Variables|Default|GetPlayer))
  (Default|Reset (Variables|Default|GetEnemy)))