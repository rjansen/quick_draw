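; BP_Samurai is a 2D Paper sprite duelist in a quick-draw duel run by GM_Duel.
; It slides in on a timeline at begin play and on Reset, and allows one attack press per round.
; Pressing during Wait shows a cross, while pressing during Draw ends the game and lunges to the attack position.
; The lunge timeline swaps in the attack sprite and reports the hit to GM_Duel, flagging whether the samurai is player-controlled.
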(event Custom|SlideIn
  (Components|Timeline|SetPlayRate (Variables|Default|GetSlideInAnimation) 2.0)
  (bind _alpha (Timeline|SlideInAnimation PlayFromStart)
    (:Update
      (Transformation|SetRelativeLocation (Variables|Default|GetPaperSprite) (Math|Vector|Lerp(Vector) (Variables|Default|GetSlideInPosition) (Variables|Default|GetSpriteDefaultPosition) _alpha) false false))))

(event Custom|Attack
  (if (not (Variables|Default|GetPressedDraw))
    (switch Utilities|FlowControl|Switch|SwitchonE_Phases (Variables|/Game/Blueprints/GM_Duel.GM_Duel_C|GetPhase (Variables|Default|GetDuelRef))
      (:NewEnumerator1
        (CallFunction|SetCrossVisibility true)
        (Variables|Default|SetPressedDraw true))
      (:NewEnumerator2
        (Variables|Default|SetPressedDraw true)
        (Default|SetGameFinished (Variables|Default|GetDuelRef))
        (Components|Timeline|SetPlayRate (Variables|Default|GetAttackAnimation) 8.0)
        (bind _alpha (Timeline|AttackAnimation PlayFromStart)
          (:Update
            (Transformation|SetRelativeLocation (Variables|Default|GetPaperSprite) (Math|Vector|Lerp(Vector) (Variables|Default|GetSpriteDefaultPosition) (Variables|/Script/Engine.SceneComponent|GetRelativeLocation (Variables|Default|GetAttackPosition)) _alpha) false false))
          (:SwitchSprite
            (CallFunction|SetSprite (Variables|Default|GetAttackSprite))
            (Default|AttackedSuccessfully (Variables|Default|GetDuelRef) (Pawn|IsPlayerControlled))))))))

(event Custom|Defeated
  (CallFunction|SetSprite (Variables|Default|GetDefeatedSprite))
  (CallFunction|SetCrossVisibility false))

(event EventBeginPlay
  (bind _asgm_duel (Utilities|Casting|CastToGM_Duel (Game|GetGameMode))
    (:then
      (Variables|Default|SetDuelRef _asgm_duel)
      (Variables|Default|SetSpriteDefaultPosition (Variables|/Script/Engine.SceneComponent|GetRelativeLocation (Variables|Default|GetPaperSprite)))
      (CallFunction|Slidein)
      (CallFunction|SetCrossVisibility false))
    (:CastFailed
      (Development|PrintString "Invalid Game Mode!"))))

(fn ConstructionScript)

(fn SetCrossVisibility
  (params (bNewVisibility :type Boolean))
  (Rendering|SetVisibility (Variables|Default|GetCross) bNewVisibility false))

(fn SetSprite
  (params (NewSprite :type Paper%20Sprite%20Object%20Reference))
  (Rendering|Components|Sprite|SetSprite (Variables|Default|GetPaperSprite) NewSprite)
  (Rendering|Material|SetMaterial (Variables|Default|GetPaperSprite) 0 "/Paper2D/TranslucentUnlitSpriteMaterial.TranslucentUnlitSpriteMaterial")
  (Rendering|SetTranslucencySortDistanceOffset (Variables|Default|GetPaperSprite) 1.0))

(fn Reset
  (CallFunction|SetSprite (Variables|Default|GetIdleSprite))
  (Variables|Default|SetPressedDraw false)
  (CallFunction|Slidein))